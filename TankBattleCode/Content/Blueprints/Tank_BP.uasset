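; Tank Blueprint that handles player camera aiming and firing input.
; On BeginPlay it passes its barrel and turret components to SetBarrelReference and SetTurrentReference.
; Azimuth input yaws a gimbal and latitude input pitches the spring arm, both as scaled local rotations per axis value.
; The Fire action calls Fire, whose logic is not defined in this graph.
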(event EventBeginPlay
  ;[1 1 1] Comment
  (Class|Tank|SetBarrelReference (Variables|Default|GetTankBarrel))
  (Class|Tank|SetTurrentReference (Variables|Default|GetTankTurrent)))

(event EventTick
  (params (DeltaSeconds :type Float%20%28single-precision%29)))

(event Input|ActionEvents|InputActionFire
  (params (Key :type Key%20Structure))
  ;[1 1 1] Input Handle
  (:Pressed
    (Class|Tank|Fire)))

(event Input|AxisEvents|InputAxisAimAzimuth
  (params (AxisValue :type Float%20%28single-precision%29))
  ;[1 1 1] Input Handle
  (Transformation|AddLocalRotation (Variables|Default|GetAzimuthGimbal) (Math|Rotator|MakeRotator 0.0 0.0 (* AxisValue 5.0)) false false))

(event Input|AxisEvents|InputAxisAimLatitude
  (params (AxisValue :type Float%20%28single-precision%29))
  ;[1 1 1] Input Handle
  (Transformation|AddLocalRotation (Variables|Default|GetSpringArm) (Math|Rotator|MakeRotator 0.0 (* AxisValue 5.0) 0.0) false false))

(fn ConstructionScript)